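; Portal actor that moves the game to a configurable level when a Character enters it.
; Overlapping the Box with a Character calls ServerTravel on MyGameInstance with TravelLevel.
; The construction script shows the TravelLevel name on the TextRender and applies PortalMaterial to the portal plane mesh.
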(event `self.Box.OnComponentBeginOverlap`
  (params (OverlappedComponent :type "PrimitiveComponent Object Reference") (OtherActor :type "Actor Object Reference") (OtherComp :type "PrimitiveComponent Object Reference") (OtherBodyIndex :type Integer) (bFromSweep :type Boolean) (SweepResult :type "HitResult Structure (by ref)"))
  (cast `Character` OtherActor)
  (bind _asmy_game_instance (cast `/Game/Blueprints/MyGameInstance` (`GameplayStatics.GetGameInstance`)))
  (`/Game/Blueprints/MyGameInstance.ServerTravel` _asmy_game_instance (`self.TravelLevel`)))

(fn `UserConstructionScript`
  (`TextRenderComponent.K2_SetText` (`self.TextRender`) (`KismetTextLibrary.Conv_StringToText` (`self.TravelLevel`)))
  (`PrimitiveComponent.SetMaterial` (`self.SM_PortalFrame_PortalPlane`) 0 (`self.PortalMaterial`)))