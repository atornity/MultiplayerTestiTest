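; TestMovingCharacter is a test character that moves by itself, starting along its forward vector.
; On each tick, only with authority, it adds movement input along the stored direction at a set speed scale.
; A short debug-drawn visibility trace looks ahead, and on a hit the surface normal becomes the new direction, turning the character away from obstacles.
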(event `self.ReceiveBeginPlay`
  (set `self.InputDirection` (`self.GetActorForwardVector`)))

(event `self.ReceiveTick`
  (params (DeltaSeconds :type "Float (single-precision)"))
  (bind _returnvalue (`self.K2_GetActorLocation`))
  (bind _inputdirection (`self.InputDirection`))
  (`/Engine/EditorBlueprintResources/ActorMacros.Switch Has Authority`
    (:`Authority`
      (`self.AddMovementInput` _inputdirection (`self.SpeedScale`))
      (bind (_outhit _returnvalue_2) (`KismetSystemLibrary.LineTraceSingle` :`Start` _returnvalue :`End` (+ _returnvalue (* _inputdirection 75.0)) :`TraceChannel` "TraceTypeQuery1" :`DrawDebugType` "ForOneFrame"))
      (if _returnvalue_2
        (set `self.InputDirection` (`.Normal` (`GameplayStatics.BreakHitResult` _outhit)))))))

(fn `UserConstructionScript`)