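; Game instance Blueprint that opens the multiplayer lobby UI and triggers server travel between levels.
; AddWidget creates the MultiplayerLobby widget for the first player controller, shows the mouse cursor and focuses the widget in Game and UI input mode.
; ServerTravel stores the requested level in NextLevel and runs a servertravel console command, appending the level name directly with no separator.
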(event `AddWidget`
  (bind _returnvalue (`GameplayStatics.GetPlayerController` 0))
  (`/Engine/EditorBlueprintResources/StandardMacros.IsValid` (`GameplayStatics.GetPlayerController` 0)
    (:`Is Valid`
      (bind _returnvalue_2 (`|CreateWidget` "/Game/Widgets/MultiplayerLobby.MultiplayerLobby_C" _returnvalue))
      (`UserWidget.AddToViewport` _returnvalue_2 0)
      (set `PlayerController.bShowMouseCursor` true _returnvalue)
      (`WidgetBlueprintLibrary.SetInputMode_GameAndUIEx` _returnvalue _returnvalue_2))))

(event `ServerTravel`
  (params (Level :type String))
  (bind _output_get (set `self.NextLevel` Level))
  (`KismetSystemLibrary.ExecuteConsoleCommand` (`KismetStringLibrary.Concat_StrStr` "servertravel " _output_get) (`GameplayStatics.GetPlayerController` 0)))